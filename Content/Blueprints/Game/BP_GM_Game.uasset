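; BP_GM_Game is the game mode that manages the player's oxygen supply and triggers game over when it runs out.
; On BeginPlay a looping timer drains Oxygen each tick by a rounded depletion speed times tick rate, clamped at zero.
; At zero it clears the timer and calls the game over event.
; AddOxygen refills up to OxygenMax, and AddMax raises that cap.
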(event Custom|AddOxygen
  (params (Amount :type Integer))
  (Variables|Default|SetOxygen (Math|Integer|Clamp(Integer) (+ (Variables|Default|GetOxygen) Amount) 0 (Variables|Default|GetOxygenMax))))

(event Custom|AddMax
  (params (Amount :type Integer))
  (Variables|Default|SetOxygenMax (+ (Variables|Default|GetOxygenMax) Amount)))

(event Custom|DrainOxygen
  (bind _output_get (Variables|Default|SetOxygen (Math|Integer|Clamp(Integer) (- (Variables|Default|GetOxygen) (Math|Float|Round (* (Variables|Default|GetdepleteSpeed) (Variables|Default|GetOxygenTickRate)))) 0 9999999)))
  (if (<= _output_get 0)
    (Utilities|Time|ClearandInvalidateTimerbyHandle (Variables|Default|GetOxygenHandle))
    (Default|CallGameOver)))

(event EventBeginPlay
  (bind _returnvalue (Utilities|Time|SetTimerbyEvent (delegate Custom|DrainOxygen) (Variables|Default|GetOxygenTickRate) true))
  (Variables|Default|SetOxygenHandle _returnvalue))

(event EventTick
  (params (DeltaSeconds :type Float%20%28single-precision%29)))

(fn ConstructionScript)