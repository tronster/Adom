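; World manager that streams an endless grid of tile chunks around the player pawn and occasionally seeds oxygen pickups.
; Delayed Tick checks fill the 3x3 neighbourhood, choosing tile classes deterministically from seeded, skewed Perlin noise.
; Chunks beyond a boxy distance threshold get pruned by destroying the nearest live tile, with a count cap trimming only the list.
; When a countdown expires, the next new chunk receives randomized oxygen and the interval grows by half.
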(event Custom|SpawnChunk
  (params (worldx :type Float%20%28double-precision%29) (worldy :type Float%20%28double-precision%29))
  ;[0.15 0.15 0.15 0.5] DEPRECATED
  (bind _exists (CallFunction|ChunkExists (Math|Float|Floor (/ worldx (Variables|Default|GetpieceWidth))) (Math|Float|Floor (/ worldy (Variables|Default|GetpieceHeight)))))
  (if (not _exists)
    (CallFunction|CreateChunk)))

(event EventBeginPlay
  (Variables|Default|SetPlayerPawn (Game|Player|GetPlayerPawn 0))
  (CallFunction|CreateStart)
  (Variables|Default|SetCountdownToOxygen (Variables|Default|GetMaxToOxygen)))

(event Collision|EventActorBeginOverlap
  (params (OtherActor :type Actor%20Object%20Reference)))

(event EventTick
  (params (DeltaSeconds :type Float%20%28single-precision%29))
  (Variables|Default|SetCountdownToOxygen (Math|Float|Clamp(Float) (- (Variables|Default|GetCountdownToOxygen) DeltaSeconds) 0.0 9999999.0))
  (Utilities|FlowControl|Delay 0.1)
  (CallFunction|PruneChunkCheck)
  (CallFunction|CreateChunkCheck))

(fn ConstructionScript)

(fn CreateStart
  (CallFunction|CreateChunk))

(fn GetBPClassatChunk
  (params (x :type Integer) (y :type Integer))
  (bind _noiseseed (LocalVariables|GetNoiseSeed))
  (bind _noisescale (LocalVariables|GetNoiseScale))
  (bind _returnvalue (+ x _noiseseed))
  (bind _returnvalue_2 (* _returnvalue _noisescale))
  (return (Utilities|Array|Get(acopy) (Variables|Default|GetTilesClassesLevel1) (Math|Float|Floor (Class|KismetAnimationLibrary|MakePerlinNoiseandRemap (+ _returnvalue_2 (+ (* (+ y (LocalVariables|GetNoiseSeed)) (LocalVariables|GetNoiseScale)) (- 1e+03 (* _returnvalue_2 23.0)))) 0.0 (Math|Conversions|ToFloat(Integer) (Utilities|Array|Length (Variables|Default|GetTilesClassesLevel1))))))))

(fn GetLocationforChunk
  (params (x :type Integer) (y :type Integer))
  (bind _returnvalue (Transformation|GetActorLocation))
  (return (Math|Vector|MakeVector (+ (.x _returnvalue) (* x (Variables|Default|GetpieceWidth))) (+ (.y _returnvalue) (* y (Variables|Default|GetpieceHeight))) 0.0)))

(fn ChunkExists
  (params (x :type Integer) (y :type Integer))
  (bind _array_element (Utilities|Array|ForEachLoopwithBreak (Variables|Default|GetActiveChunks) :!label _label)
    (:LoopBody
      (bind _output_get (LocalVariables|SetIsExist (and (== (.X (Utilities|Struct|BreakIntVector2 _array_element)) x) (== (.Y (Utilities|Struct|BreakIntVector2 _array_element)) y))))
      (if _output_get
        (goto _label Break)))
    (:Completed
      (return (LocalVariables|GetIsExist)))))

(fn CreateChunk
  (params (x :type Integer) (y :type Integer))
  (Utilities|Array|AddUnique (Variables|Default|GetActiveChunks) (Utilities|Struct|MakeIntVector2 x y))
  (bind _output (CallFunction|GetBPClassatChunk x y))
  (bind _returnvalue (Game|SpawnActorfromClass _output (Math|Transform|MakeTransform (CallFunction|GetLocationforChunk x y)) "Undefined" "MultiplyWithRoot" 0 0))
  (Utilities|Array|AddUnique (Variables|Default|GetLiveTiles) _returnvalue)
  (return _returnvalue))

(fn PruneChunkCheck
  (bind _playerpawn (Variables|Default|GetPlayerPawn))
  (bind _returnvalue (Transformation|GetActorLocation _playerpawn))
  (Utilities|FlowControl|Sequence
    (:then_0
      (LocalVariables|Setx (Math|Float|Floor (/ (.x _returnvalue) (Variables|Default|GetpieceWidth))))
      (LocalVariables|Sety (Math|Float|Floor (/ (.y _returnvalue) (Variables|Default|GetpieceHeight))))
      (bind (_arrayindex _arrayelement) (Utilities|Array|ReverseforEachLoop (Variables|Default|GetActiveChunks))
        (:LoopBody
          (if (or (> (Math|Integer|Absolute(Integer) (- (.X (Utilities|Struct|BreakIntVector2 _arrayelement)) (LocalVariables|Getx))) (LocalVariables|GetDistanceThreshold)) (> (Math|Integer|Absolute(Integer) (- (.Y (Utilities|Struct|BreakIntVector2 _arrayelement)) (LocalVariables|Gety))) (LocalVariables|GetDistanceThreshold)))
            (Actor|DestroyActor (.ReturnValue (Actor|FindNearestActor (Math|Vector|MakeVector (Math|Conversions|ToFloat(Integer) (* (.X (Utilities|Struct|BreakIntVector2 _arrayelement)) (Variables|Default|GetpieceWidth))) (Math|Conversions|ToFloat(Integer) (* (.Y (Utilities|Struct|BreakIntVector2 _arrayelement)) (Variables|Default|GetpieceHeight))) 0.0) (Variables|Default|GetLiveTiles))))
            (Utilities|Array|RemoveIndex (Variables|Default|GetActiveChunks) _arrayindex)))))
    (:then_1
      ;[0.15 0.15 0.15 0.5] Safety; but dangerous if player went back on old chunks may be on the one that is being removed.
      (if (> (Utilities|Array|Length (Variables|Default|GetActiveChunks)) (LocalVariables|GetMaxChunks))
        (Utilities|Array|RemoveIndex (Variables|Default|GetActiveChunks))))))

(fn CreateChunkCheck
  (bind _playerpawn (Variables|Default|GetPlayerPawn))
  (bind _returnvalue (Transformation|GetActorLocation _playerpawn))
  ;[0.15 0.15 0.15 0.5] Find pawn's location, adjust for width and height offset and figure out the chunk it would be in
  (LocalVariables|Setx (Math|Float|Floor (/ (+ (* (Variables|Default|GetpieceWidth) 0.5) (.x _returnvalue)) (Variables|Default|GetpieceWidth))))
  (LocalVariables|Sety (Math|Float|Floor (/ (+ (.y _returnvalue) (* (Variables|Default|GetpieceHeight) 0.5)) (Variables|Default|GetpieceHeight))))
  ;[0.15 0.15 0.15 0.5] Look at 9 squares around this one and create chunks as necessary
  (for _index (range -1 1)
    (LocalVariables|Setnx (+ _index (LocalVariables|Getx)))
    (for _index_2 (range -1 1)
      (LocalVariables|Setny (+ _index_2 (LocalVariables|Gety)))
      (bind _exists (CallFunction|ChunkExists (LocalVariables|Getnx) (LocalVariables|Getny)))
      (if (not _exists)
        (bind _chunkactor (CallFunction|CreateChunk (LocalVariables|Getnx) (LocalVariables|Getny)))
        ;[0.15 0.15 0.15 0.5] Time for oxygen placement?
        (if (<= (Variables|Default|GetCountdownToOxygen) 0.0)
          ;[0.15 0.15 0.15 0.5] Reset next oxygen spawn to be a little longer
          (bind _output_get (Variables|Default|SetMaxToOxygen (* (Variables|Default|GetMaxToOxygen) 1.5)))
          (Variables|Default|SetCountdownToOxygen _output_get)
          (CallFunction|PlaceOxygenonChunk _chunkactor))))))

(fn PlaceOxygenonChunk
  (params (ChunkActor :type Actor%20Object%20Reference))
  (bind _returnvalue (Transformation|GetActorTransform ChunkActor))
  (bind _returnvalue_2 (Game|SpawnActorfromClass "/Game/Blueprints/Pickups/BP_Oxygen.BP_Oxygen_C" (Math|Transform|MakeTransform (Math|Vector|MakeVector (+ (.x (.location _returnvalue)) (Math|Random|RandomFloatinRange 0.0 1024.0)) (+ (.y (.location _returnvalue)) (Math|Random|RandomFloatinRange 0.0 1024.0)) (+ (.z (.location _returnvalue)) 1e+01)) (Math|Rotator|MakeRotator 0.0 0.0 (Math|Random|RandomFloatinRange 0.0 3.6e+02)) "1.000000,1.000000,1.000000") "AlwaysSpawn" "MultiplyWithRoot" ChunkActor (Math|Random|RandomIntegerinRange 100 1000) 0))
  (Development|PrintString (Utilities|String|Append "OXY at: " (Utilities|String|ToString(Vector) (Transformation|GetActorLocation _returnvalue_2)))))