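; BP_CarPawn is the player-driven car, which moves through CharacterMovement and can receive oxygen.
; On BeginPlay it adds the game's Enhanced Input mapping context and caches the game mode.
; Throttle adds movement along the forward vector, while steering yaws the actor in proportion to current speed over max speed, so it cannot turn while stationary.
; AddOxygen forwards the amount to the game mode and plays a sound.
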(event Custom|AddOxygen
  (params (Amount :type Integer))
  (Default|AddOxygen (Variables|Default|GetGameModeAdom) Amount)
  (Audio|PlaySound2D "/Game/Audio/SFX_Oxygen.SFX_Oxygen" 1.0 1.0 0.0 0 0))

(event Input|EnhancedActionEvents|EnhancedInputActionIA_Throttle
  (params (ActionValue :type Float%20%28double-precision%29) (ElapsedSeconds :type Float%20%28double-precision%29) (TriggeredSeconds :type Float%20%28double-precision%29) (InputAction :type Input%20Action%20Object%20Reference :default "/Game/Input/Actions/IA_Throttle.IA_Throttle"))
  (Pawn|Input|AddMovementInput (* (Transformation|GetActorForwardVector) ActionValue) 1.0 false))

(event Input|EnhancedActionEvents|EnhancedInputActionIA_Steer
  (params (ActionValue :type Float%20%28double-precision%29) (ElapsedSeconds :type Float%20%28double-precision%29) (TriggeredSeconds :type Float%20%28double-precision%29) (InputAction :type Input%20Action%20Object%20Reference :default "/Game/Input/Actions/IA_Steer.IA_Steer"))
  (bind _charactermovement (Variables|Character|GetCharacterMovement))
  (Class|Actor|AddActorWorldRotation (Math|Rotator|MakeRotator 0.0 0.0 (* (* ActionValue (Variables|Default|GetTurnRate)) (/ (Math|Vector|VectorLength (Variables|/Script/Engine.MovementComponent|GetVelocity _charactermovement)) (Class|MovementComponent|GetMaxSpeed _charactermovement))))))

(event EventBeginPlay
  (bind _asbp_pc_game (Utilities|Casting|CastToBP_PC_Game (Game|GetPlayerController 0)))
  (Input|AddMappingContext (PlayerController|LocalPlayerSubsystems|GetEnhancedInputLocalPlayerSubsystem _asbp_pc_game) "/Game/Input/IMC_Game.IMC_Game" 0 "(bIgnoreAllPressedKeysUntilRelease=True,bForceImmediately=False,bNotifyUserSettings=False)")
  (bind _asbp_gm_game (Utilities|Casting|CastToBP_GM_Game (Game|GetGameMode))
    (:then
      (Variables|Default|SetGameModeAdom _asbp_gm_game))
    (:CastFailed
      (Development|PrintString "bad game mode" true true "(R=1.000000,G=0.660000,B=1.000000,A=1.000000)"))))

(event Collision|EventActorBeginOverlap
  (params (OtherActor :type Actor%20Object%20Reference)))

(event EventTick
  (params (DeltaSeconds :type Float%20%28single-precision%29)))

(fn ConstructionScript)